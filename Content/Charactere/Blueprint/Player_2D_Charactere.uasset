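; Player-controlled 2D Paper character that runs along the X axis, jumps and attacks through Enhanced Input, turning its sprite with movement direction.
; Tick picks idle, run, jump or fall flipbooks from movement state unless attacking.
; Attack plays a one-shot flipbook, and its finish event restores looping idle.
; HitCheck damages other overlapping player characters in Box1, but nothing in this graph calls it.
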(event `self.ReceiveBeginPlay`
  ;[0.15 0.15 0.15 0.5 50] Player_Movement
  (`EnhancedInputSubsystemInterface.AddMappingContext` (pcsubsystem `EnhancedInputLocalPlayerSubsystem` (`GameplayStatics.GetPlayerController` 0)) "/Game/Charactere/Input/IMC_Player.IMC_Player" 0 (struct)))

(event `EnhancedInput|/Game/Charactere/Input/IA_Move`
  (params (ActionValue :type "Float (double-precision)") (ElapsedSeconds :type "Float (double-precision)") (TriggeredSeconds :type "Float (double-precision)") (InputAction :type "InputAction Object Reference" :default "/Game/Charactere/Input/IA_Move.IA_Move"))
  ;[0.15 0.15 0.15 0.5 50] Player_Movement
  (:`Triggered`
    (`self.AddMovementInput` (`GameplayStatics.GetPlayerCharacter` 0) (1.0 0.0 0.0) ActionValue false)
    (if (>= ActionValue 0.0)
      (`SceneComponent.K2_SetWorldRotation` :`self` (`self.Sprite`))
      (else
        (`SceneComponent.K2_SetWorldRotation` (`self.Sprite`) (struct :`Yaw` 90.0) false false)))))

(event `EnhancedInput|/Game/Charactere/Input/IA_Jump`
  (params (ActionValue :type Boolean) (ElapsedSeconds :type "Float (double-precision)") (TriggeredSeconds :type "Float (double-precision)") (InputAction :type "InputAction Object Reference" :default "/Game/Charactere/Input/IA_Jump.IA_Jump"))
  (bind _returnvalue (`GameplayStatics.GetPlayerCharacter` 0))
  ;[0.15 0.15 0.15 0.5 50] Player_Movement
  (:`Started`
    (`self.Jump` _returnvalue))
  (:`Completed`
    (`self.StopJumping` _returnvalue)))

(event `self.ReceiveTick`
  (params (DeltaSeconds :type "Float (single-precision)"))
  ;[0.15 0.02744 0.05928 0.7159 50] Animation
  (if (not (`self.Attacking_??`))
    (`self.Update_animation`)))

(event `EnhancedInput|/Game/Charactere/Input/IA_Attack1`
  (params (ActionValue :type Boolean) (ElapsedSeconds :type "Float (double-precision)") (TriggeredSeconds :type "Float (double-precision)") (InputAction :type "InputAction Object Reference" :default "/Game/Charactere/Input/IA_Attack1.IA_Attack1"))
  (bind _sprite (`self.Sprite`))
  (:`Started`
    (`PaperFlipbookComponent.SetFlipbook` _sprite "/Game/Charactere/Sprite/Knight/Attack002/Attack3.Attack3")
    (`PaperFlipbookComponent.SetLooping` _sprite false)
    (set `self.Attacking_??` true)))

(event `self.Sprite.OnFinishedPlaying`
  (`PaperFlipbookComponent.SetFlipbook` (`self.Sprite`) "/Game/Charactere/Sprite/Knight/Idle/Idle1.Idle1")
  (`self.Restart_Anim`)
  (set `self.Attacking_??` false))

(fn `HitCheck`
  (for _array_element (`PrimitiveComponent.GetOverlappingActors` (`self.Box1`) "Player_2D_Charactere_C")
    (if (!= _array_element (`GameplayStatics.GetPlayerCharacter` 0))
      (`GameplayStatics.ApplyDamage` _array_element (`self.Base Damage`)))))

(fn `Restart_Anim`
  (bind _sprite (`self.Sprite`))
  (`PaperFlipbookComponent.SetLooping` _sprite true)
  (if (not (`PaperFlipbookComponent.IsPlaying` _sprite))
    (`PaperFlipbookComponent.Play` (`self.Sprite`))))

(fn `Update_animation`
  (bind (_returnvalue_x _returnvalue_y _returnvalue_z) (`KismetMathLibrary.BreakVector` (`self.GetVelocity`)))
  (bind _charactermovement (`self.CharacterMovement`))
  (if (`NavMovementInterface.IsFalling` _charactermovement)
    (if (> _returnvalue_z 0.0)
      (`PaperFlipbookComponent.SetFlipbook` (`self.Sprite`) "/Game/Charactere/Sprite/Knight/Jump/Jump1.Jump1")
      (else
        (`PaperFlipbookComponent.SetFlipbook` (`self.Sprite`) "/Game/Charactere/Sprite/Knight/Jump/Fall1.Fall1")))
    (elif (> (`KismetMathLibrary.VSize` (`MovementComponent.Velocity` _charactermovement)) 0.0)
      (`PaperFlipbookComponent.SetFlipbook` (`self.Sprite`) "/Game/Charactere/Sprite/Knight/Run/Run1.Run1")
      (else
        (`PaperFlipbookComponent.SetFlipbook` (`self.Sprite`) "/Game/Charactere/Sprite/Knight/Idle/Idle1.Idle1")))))

(fn `UserConstructionScript`)